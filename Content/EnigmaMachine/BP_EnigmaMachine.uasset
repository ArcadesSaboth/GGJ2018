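; Enigma machine Blueprint that maps physical keyboard input onto its 26 child-actor keys.
; BeginPlay gathers the key components into an array, which AnyKey events search for a BP_EnigmaKey with a matching key.
; A press calls PressKey on the match, while a release calls ReleaseKey through the press loop's cast reference.
; A separate MovePressedKeyMesh graph, unused by these events, slides a mesh with a timeline.
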(event `self.ReceiveBeginPlay`
  (set `self.KeysArray` (`|MakeArray` (`self.BP_EnigmaKey_A`) (`self.ChildActor`) (`self.ChildActor1`) (`self.ChildActor2`) (`self.ChildActor3`) (`self.ChildActor4`) (`self.ChildActor5`) (`self.ChildActor6`) (`self.ChildActor7`) (`self.ChildActor8`) (`self.ChildActor9`) (`self.ChildActor10`) (`self.ChildActor11`) (`self.ChildActor12`) (`self.ChildActor13`) (`self.ChildActor14`) (`self.ChildActor15`) (`self.ChildActor16`) (`self.ChildActor17`) (`self.ChildActor18`) (`self.ChildActor19`) (`self.ChildActor20`) (`self.ChildActor21`) (`self.ChildActor22`) (`self.ChildActor23`) (`self.ChildActor24`))))

(event `Key|AnyKey`
  (params (Key :type "Key Structure"))
  (:`Pressed`
    (for _array_element (`self.KeysArray`)
      (bind _asbp_enigma_key (cast `/Game/EnigmaMachine/BP_EnigmaKey` (`ChildActorComponent.ChildActor` _array_element)))
      (if (== (`/Game/EnigmaMachine/BP_EnigmaKey.KeyPressed` _asbp_enigma_key) Key)
        (`|ExecutionSequence`
          (:`then_0`
            (`/Game/EnigmaMachine/BP_EnigmaKey.PressKey` _asbp_enigma_key))
          (:`then_1`
            (break))))))
  (:`Released`
    (for _array_element_2 (`self.KeysArray`)
      (bind _asbp_enigma_key_2 (cast `/Game/EnigmaMachine/BP_EnigmaKey` (`ChildActorComponent.ChildActor` _array_element_2)))
      (if (== (`/Game/EnigmaMachine/BP_EnigmaKey.KeyPressed` _asbp_enigma_key_2) Key)
        (`|ExecutionSequence`
          (:`then_0`
            (`/Game/EnigmaMachine/BP_EnigmaKey.ReleaseKey` _asbp_enigma_key))
          (:`then_1`
            (break)))))))

(fn `UserConstructionScript`)