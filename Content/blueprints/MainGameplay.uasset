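; MainGameplay is a gameplay Blueprint that creates the main screen UI and relays card events to it.
; On BeginPlay it creates a MainScreen widget for the first player controller, stores it as MainGUI and adds it to the viewport.
; OnCardSpawn and OnCardDeleted forward to that widget's Spawn and RemoveCard.
; Tick prints a debug "Hello" every frame, shown on screen only while MainGUI is valid.
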(event `self.ReceiveBeginPlay`
  (bind _returnvalue (`|CreateWidget` "/Game/UI/MainScreen.MainScreen_C" (`GameplayStatics.GetPlayerController` 0)))
  (bind _output_get (set `self.mainGUI` _returnvalue))
  (`UserWidget.AddToViewport` _output_get 0))

(event `self.ReceiveTick`
  (params (DeltaSeconds :type "Float (single-precision)"))
  (`KismetSystemLibrary.PrintString` "Hello" (`KismetSystemLibrary.IsValid` (`self.mainGUI`))))

(event `self.OnCardDeleted`
  (params (cardIndex :type Integer))
  (`/Game/UI/MainScreen.RemoveCard` (`self.mainGUI`) cardIndex))

(event `self.OnCardSpawn`
  (params (entry :type "CardEntry Structure (by ref)"))
  (`/Game/UI/MainScreen.Spawn` (`self.mainGUI`) entry))

(fn `UserConstructionScript`)