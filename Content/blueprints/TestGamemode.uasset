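; Test game mode for a word card game that shows the cursor and a MainScreen widget, then keeps timed word cards topped up.
; BeginPlay parses a comma-separated string into a lowercase word database, and SpawnCards draws random words to fill ActualCards toward SpawnCount.
; Tick advances card timers, queues expired cards for removal from the array and widget, then respawns.
; Fade length scales with the length of a separately drawn random word.
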(event `self.ReceiveBeginPlay`
  (bind _returnvalue (`GameplayStatics.GetPlayerController` 0))
  (set `PlayerController.bShowMouseCursor` true _returnvalue)
  (bind _returnvalue_2 (`|CreateWidget` "/Game/UI/MainScreen.MainScreen_C" _returnvalue))
  (bind _output_get (set `self.mainScreen` _returnvalue_2))
  (`UserWidget.AddToViewport` _output_get 0)
  (`self.AutoInitWords`)
  (`self.SpawnCards`))

(event `self.ReceiveTick`
  (params (DeltaSeconds :type "Float (single-precision)"))
  (`self.ProcessTick` DeltaSeconds))

(fn `AutoInitWords`
  (bind _output_get (set `self.wordDatabase` (`KismetStringLibrary.ParseIntoArray` (`self.auto`) ",")))
  (for (_array_element _array_index) _output_get
    (`KismetArrayLibrary.Array_Set` _output_get _array_index (`KismetStringLibrary.ToLower` _array_element))))

(fn `GenerateCardTimer`
  (params (word :type String))
  (returns (time :type "Float (double-precision)"))
  (return (* (`KismetStringLibrary.Len` word) 2.0)))

(fn `ProcessTick`
  (params (deltaTime :type "Float (double-precision)"))
  (locals (pendingDeletionIndex :type "Array of Integer") (pendingDeletionElements :type "Array of Integer"))
  (bind _actualcards (`self.actualCards`))
  (`|ExecutionSequence`
    (:`then_0`
      (for (_array_element _array_index) _actualcards
        (bind _returnvalue (+ (`.timer_10_EB2F50014FDCBA6BEE0A9C9587A88504` (break `/Game/blueprints/CardEntryTemp` _array_element)) deltaTime))
        (`KismetArrayLibrary.Array_Set` _actualcards _array_index (make `/Game/blueprints/CardEntryTemp` (break `/Game/blueprints/CardEntryTemp` _array_element) (`.word_5_31CE3DCC4B198518D0D05AAEDDA2B1CB` (break `/Game/blueprints/CardEntryTemp` _array_element)) (`.fadeLength_8_9B8D91E547A3E147823E69B21D068994` (break `/Game/blueprints/CardEntryTemp` _array_element)) _returnvalue))
        (if (> _returnvalue (`.fadeLength_8_9B8D91E547A3E147823E69B21D068994` (break `/Game/blueprints/CardEntryTemp` _array_element)))
          (`KismetArrayLibrary.Array_Add` (`local.pendingDeletionIndex`) _array_index))))
    (:`then_1`
      (for (_array_element_2 _array_index_2) (`local.pendingDeletionIndex`)
        (`/Game/UI/MainScreen.RemoveCard` (`self.mainScreen`) _array_element_2)
        (`KismetArrayLibrary.Array_Remove` _actualcards _array_index_2))
      (`self.SpawnCards`))))

(fn `SpawnCards`
  (locals (howMany :type Integer))
  (bind _worddatabase (`self.wordDatabase`))
  (bind _output (`|GetArrayItem` _worddatabase (`KismetMathLibrary.RandomIntegerInRange` 0 (`KismetArrayLibrary.Array_Length` _worddatabase))))
  (for _ (range (`KismetArrayLibrary.Array_Length` (`self.actualCards`)) (+ (`self.spawnCount`) 1))
    (bind _time (`self.GenerateCardTimer` _output))
    (`KismetArrayLibrary.Array_Add` (`self.actualCards`) (make `/Game/blueprints/CardEntryTemp` (`self.usedIndex`) _output _time))))

(fn `UserConstructionScript`)