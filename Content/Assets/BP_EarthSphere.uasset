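; BP_EarthSphere is an Earth sphere Blueprint that animates a group of toy soldiers, ToySoldiersA.
; Separate forward and backward timelines set its relative yaw and Z position on each update, without sweep.
; Custom events or the 1 and 2 keys play the matching timeline from the start.
; The forward event for ToySoldiersB is an empty stub, and that component's reference is unused.
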(event `MoveSoldiersA_Forward`
  (bind _toysoldiers_a (`self.ToySoldiers_A`))
  (bind (_direction _rot_z _trans_z) (`Timeline|Timeline_01_Forward` :!via `PlayFromStart` :!label _label)
    (:`Update`
      (`SceneComponent.K2_SetRelativeRotation` _toysoldiers_a (`KismetMathLibrary.MakeRotator` 0.0 0.0 _rot_z) false false)
      (`SceneComponent.K2_SetRelativeLocation` _toysoldiers_a (`KismetMathLibrary.MakeVector` 0.0 0.0 _trans_z) false false))))

(event `MoveSoldiersB_Forward`)

(event `Key|One`
  (params (Key :type "Key Structure"))
  (:`Pressed`
    (goto _label :!via `PlayFromStart`)))

(event `MoveSoldiersA_Backwards`
  (bind _toysoldiers_a (`self.ToySoldiers_A`))
  (bind (_direction _rot_z _trans_z) (`Timeline|Timeline_0` :!via `PlayFromStart` :!label _label_2)
    (:`Update`
      (`SceneComponent.K2_SetRelativeRotation` _toysoldiers_a (`KismetMathLibrary.MakeRotator` 0.0 0.0 _rot_z) false false)
      (`SceneComponent.K2_SetRelativeLocation` _toysoldiers_a (`KismetMathLibrary.MakeVector` 0.0 0.0 _trans_z) false false))))

(event `Key|Two`
  (params (Key :type "Key Structure"))
  (:`Pressed`
    (goto _label_2 :!via `PlayFromStart`)))

(fn `UserConstructionScript`)